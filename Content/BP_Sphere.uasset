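; BP_Sphere is an actor that generates points automatically in what appears to be a clicker game, playing an axe creation sound on BeginPlay.
; Tick accumulates a timer that, every few seconds, plays a hit sound and resets.
; Each cycle then adds PointValue to BP_GameMode's points and click count, and refreshes the widget's progress bar toward the next-actor threshold.
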(event `self.ReceiveBeginPlay`
  (`GameplayStatics.PlaySound2D` "/Game/Audio/create_axe.create_axe" 1.0 1.0 0.0 null null))

(event `self.ReceiveTick`
  (params (DeltaSeconds :type "Float (single-precision)"))
  (bind _output_get (set `self.Timer` (+ DeltaSeconds (`self.Timer`))))
  (if (>= _output_get 3.0)
    (`GameplayStatics.PlaySound2D` "/Game/Audio/hit_axe.hit_axe" 1.0 1.0 0.0 null null)
    (set `self.Timer` 0.0)
    (bind _asbp_game_mode (cast `/Game/BP_GameMode` (`GameplayStatics.GetGameMode`)))
    (`/Game/BP_GameMode.AddPoints` _asbp_game_mode (`self.PointValue`))
    (bind _output_get_2 (set `/Game/BP_GameMode.Clicks` (+ (`/Game/BP_GameMode.Clicks` _asbp_game_mode) (`self.PointValue`)) _asbp_game_mode))
    (`/Game/BP_UserWidget.SetProgressBar` (`/Game/BP_GameMode.Widget` _asbp_game_mode) (`KismetMathLibrary.Conv_IntToDouble` _output_get_2) (`KismetMathLibrary.Conv_IntToDouble` (`/Game/BP_GameMode.ClicksToNewActor` _asbp_game_mode)))))

(fn `UserConstructionScript`)